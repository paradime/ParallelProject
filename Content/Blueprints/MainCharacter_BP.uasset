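; Main character Blueprint that implements a directional roll.
; The Roll event plays a timeline that, on each update, turns player 0's controller toward the XMove/YMove vector, falling back to +X when both are zero.
; The timeline's Distance track scales that vector and feeds UpdateRollLocation.
; IsRolling is true while the timeline updates and clears when it finishes.
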(event EventBeginPlay)

(event Collision|EventActorBeginOverlap
  (params (OtherActor :type Actor%20Object%20Reference)))

(event EventTick
  (params (DeltaSeconds :type Float%20%28single-precision%29)))

(event EventRoll
  (bind _distance (Timeline|Roll_Location PlayFromStart)
    (:Update
      (Variables|Default|SetbIsRolling true)
      (if (and (== (Variables|Default|GetXMove) 0.0) (== (Variables|Default|GetYMove) 0.0))
        (Variables|Default|SetXMove 1.0))
      (Pawn|SetControlRotation (Pawn|GetController (Game|Player|GetPlayerPawn 0)) (Math|Conversions|RotationFromXVector (Math|Vector|MakeVector (Variables|Default|GetXMove) (Variables|Default|GetYMove) 0.0)))
      (Class|MainCharacter|UpdateRollLocation (* _distance (Variables|Default|GetXMove)) (* (Variables|Default|GetYMove) _distance)))
    (:Finished
      (Variables|Default|SetbIsRolling false))))

(fn ConstructionScript)